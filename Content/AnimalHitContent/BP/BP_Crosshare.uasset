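; BP_Crosshare is an interactable actor that lets the first-person character buy a crosshair.
; Box overlap enables input, caches the character and opens a gate, while end overlap disables input and closes it.
; Pressing Interact through the open gate calls BuyCrosshair on the character.
; Success destroys the actor, while failure prints a Czech message saying the player has no apple.
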(event OnComponentBeginOverlap(Box)
  (params (OverlappedComponent :type Primitive%20Component%20Object%20Reference) (OtherActor :type Actor%20Object%20Reference) (OtherComp :type Primitive%20Component%20Object%20Reference) (OtherBodyIndex :type Integer) (bFromSweep :type Boolean) (SweepResult :type Hit%20Result%20Structure%20%28by%20ref%29))
  ;[1 1 1] while player in collision with item → enable pickup
  (Input|EnableInput (Game|GetPlayerController 0))
  (Variables|Default|SetisPlayerClose true)
  (bind _asbp_first_person_character (Utilities|Casting|CastToBP_FirstPersonCharacter OtherActor))
  (Utilities|FlowControl|Gate true) ; enters at Open
)

(event OnComponentEndOverlap(Box)
  (params (OverlappedComponent :type Primitive%20Component%20Object%20Reference) (OtherActor :type Actor%20Object%20Reference) (OtherComp :type Primitive%20Component%20Object%20Reference) (OtherBodyIndex :type Integer))
  ;[1 1 1] while player in collision with item → enable pickup
  (Input|DisableInput (Game|GetPlayerController 0))
  (Variables|Default|SetisPlayerClose false)
  (Utilities|Casting|CastToBP_FirstPersonCharacter OtherActor)
  (Utilities|FlowControl|Gate true) ; enters at Close
)

(event Input|ActionEvents|InputActionInteract
  (params (Key :type Key%20Structure))
  ;[1 1 1] while player in collision with item → enable pickup
  (:Pressed
    (Utilities|FlowControl|Gate true
      (:Exit
        (bind _successfully_bought (Default|BuyCrosshair (stale OnComponentBeginOverlap(Box) _asbp_first_person_character)))
        (if _successfully_bought
          (Actor|DestroyActor)
          (else
            (Development|PrintString "Nemáš jablko")))))))

(fn ConstructionScript)