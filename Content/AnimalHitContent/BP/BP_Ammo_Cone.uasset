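; BP_Ammo_Cone is a pine cone ammo pickup that refills the first-person character's cone ammo.
; Overlapping its sphere adds a fixed amount to the character's AmmoCone, capped at a maximum, and prints the new count.
; Rather than being destroyed, it hides its mesh and disables collision, then reappears after a short delay to act as a respawning pickup.
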(event OnComponentBeginOverlap(Sphere)
  (params (OverlappedComponent :type Primitive%20Component%20Object%20Reference) (OtherActor :type Actor%20Object%20Reference) (OtherComp :type Primitive%20Component%20Object%20Reference) (OtherBodyIndex :type Integer) (bFromSweep :type Boolean) (SweepResult :type Hit%20Result%20Structure%20%28by%20ref%29))
  (bind _staticmesh (Variables|Default|GetStaticMesh))
  ;[1 1 1] Munice - šiška (spawnování nových, ničení použitých)
  (bind _asbp_first_person_character (Utilities|Casting|CastToBP_FirstPersonCharacter OtherActor))
  (if (<= (Variables|/Game/AnimalHitContent/Player/FirstPerson/Blueprints/BP_FirstPersonCharacter.BP_FirstPersonCharacter_C|GetAmmoCone _asbp_first_person_character) 15)
    (bind _output_get (Variables|/Game/AnimalHitContent/Player/FirstPerson/Blueprints/BP_FirstPersonCharacter.BP_FirstPersonCharacter_C|SetAmmoCone _asbp_first_person_character (+ (Variables|/Game/AnimalHitContent/Player/FirstPerson/Blueprints/BP_FirstPersonCharacter.BP_FirstPersonCharacter_C|GetAmmoCone _asbp_first_person_character) 5)))
    (else
      (Variables|/Game/AnimalHitContent/Player/FirstPerson/Blueprints/BP_FirstPersonCharacter.BP_FirstPersonCharacter_C|SetAmmoCone _asbp_first_person_character 20)))
  (Development|PrintString (Utilities|String|ToString(Integer) _output_get) true true "(R=0.254902,G=0.098039,B=0.019608,A=1.000000)")
  (Rendering|SetVisibility _staticmesh false false)
  (Collision|SetActorEnableCollision false)
  (Utilities|FlowControl|Delay 5.0)
  (Rendering|SetVisibility _staticmesh true false)
  (Collision|SetActorEnableCollision true))

(fn ConstructionScript)